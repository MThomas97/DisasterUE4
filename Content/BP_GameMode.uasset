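; Game mode for a four-player local game with forts, running a state machine for menu, play, dice rolls, pause and end.
; BeginPlay spawns cameras, assigns forts to players by index, creates extra local players and shows the main menu.
; StartGame initialises each controller's character, then Tick runs the match timer and interrupts play with dice screens at even intervals.
; State changes blend the first player's view between orbit, in-game and dice cameras.
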(event `self.ReceiveBeginPlay`
  (`|ExecutionSequence`
    (:`then_0`
      (bind _returnvalue (`|SpawnActorFromClass` "/Game/IngameCamera.IngameCamera_C" (`KismetMathLibrary.MakeTransform` (0.0 0.0 0.0)) "AlwaysSpawn" "OverrideRootScale" null null))
      (set `self.IngameCamera` _returnvalue)
      (bind _returnvalue_2 (`|SpawnActorFromClass` "/Game/UI/OrbitCamera.OrbitCamera_C" (`KismetMathLibrary.MakeTransform` (0.0 0.0 0.0)) "Undefined" "OverrideRootScale" null null))
      (set `self.OrbitCamera` _returnvalue_2)
      (bind _outactors (`GameplayStatics.GetAllActorsOfClass` "/Game/Fort.Fort_C"))
      (bind _output_get (set `self.Forts` _outactors))
      (for (_array_element _array_index) _output_get
        (set `/Game/Fort.OwningPlayerIndex` _array_index _array_element)
        (bind _returnvalue_3 (`|SpawnActorFromClass` "/Script/Engine.CameraActor" (`KismetMathLibrary.MakeTransform` (0.0 0.0 4000.0) (struct :`Pitch` -90.0)) "AlwaysSpawn" "OverrideRootScale" null null))
        (bind _output_get_2 (set `self.DiceMenuCamera` _returnvalue_3))
        (`CameraComponent.SetConstraintAspectRatio` (`CameraActor.CameraComponent` _output_get_2) false)))
    (:`then_1`
      ;[1 1 1] Big poopie, but lets just create all the players immediately
      (for _index (range 1 4)
        (`GameplayStatics.CreatePlayer` _index)))
    (:`then_2`
      ;[1 1 1] create menu
      (bind _returnvalue_4 (`|CreateWidget` "/Game/UI/Widgets/UMG_MainMenu.UMG_MainMenu_C"))
      (bind _output_get_3 (set `self.Menu` _returnvalue_4))
      (`UserWidget.AddToViewport` _output_get_3 0)
      (add `/Game/UI/Widgets/UMG_MainMenu.StartGame` _output_get_3 (`|CreateDelegate` :!event `StartGame`))
      (`self.ShowMenu`))))

(event `ShowMenu`
  ;[1 1 1] Show Menu
  (set `self.CurrentGameState` "NewEnumerator0")
  (`/Game/UI/Widgets/UMG_MainMenu.ShowMenu` (`self.Menu`))
  (`PlayerController.SetViewTargetWithBlend` (`GameplayStatics.GetPlayerController` 0) (`self.OrbitCamera`) 2.0 "VTBlend_Cubic" 0.0 false))

(event `StartGame`
  ;[1 1 1] Start game state
  (`PlayerController.SetViewTargetWithBlend` (`GameplayStatics.GetPlayerController` 0) (`self.IngameCamera`) 2.0 "VTBlend_Cubic" 0.0 false)
  (set `self.CurrentGameState` "NewEnumerator1")
  (set `self.GameTimer` 0.0)
  (for _index (range 4)
    (bind _asbase_player_controller (cast `/Game/BasePlayerController` (`GameplayStatics.GetPlayerController` _index)))
    (bind _character (`/Game/BasePlayerController.InitialiseCharacter` _asbase_player_controller (`|GetArrayItem` (`self.CharacterOptions`) _index)))
    (`KismetArrayLibrary.Array_Add` (`self.InGameCharacters`) _character)))

(event `StartDiceState`
  (bind _rollingplayer (`self.RollingPlayer`))
  ;[1 1 1] Start Dice State
  (set `self.CurrentGameState` "NewEnumerator2")
  (bind _returnvalue (`|CreateWidget` "/Game/UI/Widgets/umg_DiceMenu.umg_DiceMenu_C"))
  (`UserWidget.AddToViewport` _returnvalue 0)
  (`/Engine/EditorBlueprintResources/StandardMacros.IncrementInt` _rollingplayer
    (:`  `
      (`/Game/UI/Widgets/umg_DiceMenu.SetupScreen` _returnvalue _rollingplayer)
      (`PlayerController.SetViewTargetWithBlend` (`GameplayStatics.GetPlayerController` 0) (`self.DiceMenuCamera`) 2.0 "VTBlend_Cubic" 0.0 false))))

(event `self.ReceiveTick`
  (params (DeltaSeconds :type "Float (single-precision)"))
  (switch `/Game/GameStates` (`self.CurrentGameState`)
    (:`NewEnumerator1`
      ;[1 1 1] Ingame game state
      (bind _output_get (set `self.GameTimer` (+ (`self.GameTimer`) DeltaSeconds)))
      (if (> _output_get (`self.GameTimerMax`))
        (set `self.CurrentGameState` "NewEnumerator3")
        (`self.PrintGameState(DEBUG)`)
        (elif (`self.IsTimeToDisplayDice`)
          (`self.StartDiceState`))))))

(event `ResumeFromDiceState`
  (params (DiceNumber :type Integer))
  ;[1 1 1] Resume After Dice
  ;;[1 1 1] Do dice stuff
  (`/Engine/EditorBlueprintResources/StandardMacros.IncrementInt` (`self.NumberOfRolls`)
    (:`  `
      (set `self.CurrentGameState` "NewEnumerator1")
      (`PlayerController.SetViewTargetWithBlend` (`GameplayStatics.GetPlayerController` 0) (`self.IngameCamera`) 2.0 "VTBlend_Cubic" 0.0 false))))

(event `OpenPauseMenu`
  ;[1 1 1] Open/Close Menu
  (switch `/Game/GameStates` (`self.CurrentGameState`)
    (:`NewEnumerator1`
      _)
    (:`NewEnumerator5`
      _))
  (bind _output_get (set `self.Paused` (not (`self.Paused`))))
  (set `self.CurrentGameState` (select `bool` _output_get :`false` "NewEnumerator1" :`true` "NewEnumerator5" :!type "/Game/GameStates Enum"))
  (`self.PrintGameState(DEBUG)`))

(fn `GetFort`
  (params (PlayerID :type Integer))
  (returns (Fort :type "/Game/Fort Object Reference"))
  (if (> (`KismetArrayLibrary.Array_Length` (`self.Forts`)) PlayerID)
    (return (`|GetArrayItem` (`self.Forts`) PlayerID))
    (else
      (`KismetSystemLibrary.PrintText` "Out of range"))))

(fn `IsTimeToDisplayDice`
  (returns (ReturnValue :type Boolean))
  (return (> (`self.GameTimer`) (* (`self.NumberOfRolls`) (/ (`self.GameTimerMax`) (`KismetMathLibrary.Conv_IntToDouble` (`self.NumberOfRollsMax`)))))))

(fn `SetFortColour`
  (params (PlayerID :type Integer) (Colour :type "Color Structure"))
  (bind _fort (`self.GetFort` PlayerID))
  (`/Engine/EditorBlueprintResources/StandardMacros.IsValid` _fort
    (:`Is Valid`
      (`/Game/Fort.SetFortTapeColour` _fort (`KismetMathLibrary.Conv_ColorToLinearColor` Colour)))))

(fn `UserConstructionScript`)